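; Arcane Shards gameplay ability that shows a magic circle and, on an input press, targets the location under the mouse.
; It turns the avatar to face that spot, spawns a BP_PointCollection for randomly rotated ground points, and plays the cast montage.
; The montage's gameplay event hides the circle and starts a looping timer that fires a shard GameplayCue point by point, then cleans up and ends the ability.
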(event `self.K2_ActivateAbility`
  (`|ExecutionSequence`
    (:`then_0`
      (message `PlayerInterface.ShowMagicCircle` (`self.GetAvatarActorFromActorInfo`) null))
    (:`then_1`
      (`AbilityTask_WaitInputPress.WaitInputPress` false
        (:`OnPress`
          (bind (_asynctaskproxy _datahandle) (`TargetDataUnderMouse.CreateTargetDataUnderMouse`)
            (:`ValidData`
              (bind _output_get (set `self.MouseHitLocation` (`.Location` (`GameplayStatics.BreakHitResult` (`AbilitySystemBlueprintLibrary.GetHitResultFromTargetData` _datahandle)))))
              (message `CombatInterface.UpdateFacingTarget` (`self.GetAvatarActorFromActorInfo`) _output_get)
              (bind _returnvalue (`|SpawnActorFromClass` "/Game/Blueprints/AbilitySystem/Aura/GamePlayAbilities/Arcane/ArcaneShards/BP_PointCollection.BP_PointCollection_C" (`KismetMathLibrary.MakeTransform` (`self.MouseHitLocation`)) "Undefined" "MultiplyWithRoot" null null))
              (set `self.Point Collection` _returnvalue)
              (set `self.GroundPoints` (`PointCollection.GetGroundPoints` (`self.Point Collection`) (`self.MouseHitLocation`) (`self.Num Points`) (`KismetMathLibrary.RandomFloatInRange` 0.0 360.0)))
              (`AbilityTask_PlayMontageAndWait.CreatePlayMontageAndWaitProxy` "None" "/Game/Assets/Characters/Aura/Animations/Abilities/Cast_ArcaneShards_Montage.Cast_ArcaneShards_Montage" 1.0 "None" false
                (:`then`
                  (`AbilityTask_WaitGameplayEvent.WaitGameplayEvent` (struct :`TagName` "Event.Montage.ArcaneShards") null true
                    (:`EventReceived`
                      (bind _returnvalue_2 (`KismetSystemLibrary.K2_SetTimerDelegate` (delegate `在点处生成`) 0.1 true))
                      (set `self.ShardSpawnTimer` _returnvalue_2)
                      (message `PlayerInterface.HideMagicCircle` (`self.GetAvatarActorFromActorInfo`))
                      (`self.在点处生成`))))))))))))

(event `在点处生成`
  (if (< (`self.Count`) (`self.Num Points`))
    (set `self.ShardSpawnLocation` (`SceneComponent.K2_GetComponentLocation` (`|GetArrayItem` (`self.GroundPoints`) (`self.Count`))))
    (`/Engine/EditorBlueprintResources/StandardMacros.IncrementInt` (`self.Count`)
      (:`  `
        (`self.K2_ExecuteGameplayCueWithParams` (struct :`TagName` "GameplayCue.ArcaneShards") (`AbilitySystemBlueprintLibrary.MakeGameplayCueParameters` 0.0 0.0 (struct) (struct) (struct) (struct) (struct) (`self.ShardSpawnLocation`)))))
    (else
      (`KismetSystemLibrary.K2_ClearAndInvalidateTimerHandle` (`self.ShardSpawnTimer`))
      (`KismetSystemLibrary.Delay` 0.2)
      (`Actor.K2_DestroyActor` (`self.Point Collection`))
      (`KismetArrayLibrary.Array_Clear` (`self.GroundPoints`))
      (`self.K2_EndAbility`))))