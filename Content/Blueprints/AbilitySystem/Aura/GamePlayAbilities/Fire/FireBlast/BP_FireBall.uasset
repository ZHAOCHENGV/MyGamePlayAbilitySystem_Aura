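; FireBlast ability fireball that flies out and back, then explodes on nearing its ReturnToActor.
; On the server, one timeline lerps it forward to an apex, then a second lerps it toward that actor's live location.
; Within explode distance, it calls OnHit, applies radial damage with 45-degree-pitched knockback to nearby live players except itself and its owner, then destroys itself.
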(event `self.StartOutgoingTimeline`
  (`/Engine/EditorBlueprintResources/ActorMacros.Switch Has Authority`
    (:`Authority`
      ; 存储初始位置和顶点位置
      (set `self.InitialLocation` (`self.K2_GetActorLocation`))
      (set `self.ApexLocation` (+ (`self.InitialLocation`) (* (`self.GetActorForwardVector`) (`self.TravelDistance`))))
      (bind (_direction `_新建轨道_0`) (`Timeline|时间轴`)
        (:`Update`
          (`self.K2_SetActorLocation` (`KismetMathLibrary.VLerp` (`self.InitialLocation`) (`self.ApexLocation`) `_新建轨道_0`)))
        (:`Finished`
          (bind (_direction_2 `_新建轨道_0_2`) (`Timeline|时间轴_0`)
            (:`Update`
              (`self.K2_SetActorLocation` (`KismetMathLibrary.VLerp` (`self.ApexLocation`) (`self.K2_GetActorLocation` (`self.ReturnToActor`)) `_新建轨道_0_2`))
              (if (`self.IsWithinExplodeDistance`)
                (`self.OnHit`)
                (`AuraAbilitySystemLibrary.SetIsRadialDamageEffectParam` (`self.ExplosionDamageParams`) true (`self.Radial Damage Inner Radius`) (`self.Radial Damage Outer Radius`) (`self.K2_GetActorLocation`))
                (bind _outoverlappingactors (`AuraAbilitySystemLibrary.GetLivePlayersWithinRadius` self (`|MakeArray` (`self.GetOwner`) self :!type "Actor Object Reference") (`self.Radial Damage Outer Radius`) (`self.K2_GetActorLocation`)))
                (for _array_element _outoverlappingactors
                  (`AuraAbilitySystemLibrary.SetTargetEffectParamsASC` (`self.ExplosionDamageParams`) (`AbilitySystemBlueprintLibrary.GetAbilitySystemComponent` _array_element))
                  (set `self.KnockbackDirection` (- (`self.K2_GetActorLocation` _array_element) (`self.K2_GetActorLocation`)))
                  (`AuraAbilitySystemLibrary.SetKnockbackDirection` (`self.ExplosionDamageParams`) (`self.OverrideKnockbackPitch`) (`self.KnockbackMagnitude`))
                  (`AuraAbilitySystemLibrary.SetDeathImpulseDirection` (`self.ExplosionDamageParams`) (- (`self.K2_GetActorLocation`) (`self.K2_GetActorLocation`)) (`self.DeathImpulseMagnitude`))
                  (`AuraAbilitySystemLibrary.ApplyDamageEffect` (`self.ExplosionDamageParams`)))
                (`self.K2_DestroyActor`)))))))))

(fn `IsWithinExplodeDistance`
  (returns (ReturnValue :type Boolean))
  (return (<= (`KismetMathLibrary.VSize` (- (`self.K2_GetActorLocation`) (`self.K2_GetActorLocation` (`self.ReturnToActor`)))) (`self.ExplodeDistance`))))

(fn `OverrideKnockbackPitch`
  (returns (ReturnValue :type "Vector Structure"))
  (return (`KismetMathLibrary.GetForwardVector` (`KismetMathLibrary.MakeRotator` (.roll (`KismetMathLibrary.MakeRotFromX` (`self.KnockbackDirection`))) 45.0 (.yaw (`KismetMathLibrary.MakeRotFromX` (`self.KnockbackDirection`)))))))

(fn `UserConstructionScript`)