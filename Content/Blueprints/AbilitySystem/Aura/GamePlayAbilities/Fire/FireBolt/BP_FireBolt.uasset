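; Fire Bolt projectile actor for the Aura fire ability, with a fail-safe against hovering in place when its homing target dies or is missing.
; Each Tick it compares its location to the previous frame's, treating movement at or below a minimum per-frame distance as stalled.
; A stalled bolt plays the impact sound and Niagara fire explosion at its location, then destroys itself.
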(event `self.ReceiveTick`
  (params (DeltaSeconds :type "Float (single-precision)"))
  ; 为了防止当归回目标死亡或者不存在时，Actor会在目标位置悬浮
  (set `self.上一帧位置` (`self.当前帧位置`))
  (set `self.当前帧位置` (`self.K2_GetActorLocation`))
  (if (<= (`KismetMathLibrary.VSize` (- (`self.当前帧位置`) (`self.上一帧位置`))) (`self.每帧最短距离`))
    (`GameplayStatics.SpawnSoundAtLocation` "/Game/Assets/Sounds/Abilities/FireBolt/sfx_FireBolt_Impact.sfx_FireBolt_Impact" (`self.当前帧位置`) (struct) 1.0 1.0 0.0 null null)
    (`NiagaraFunctionLibrary.SpawnSystemAtLocation` "/Game/Assets/Effects/Projectiles/FireExplosion/NS_FireExplosion1.NS_FireExplosion1" (`self.当前帧位置`))
    (`self.K2_DestroyActor`)))

(fn `UserConstructionScript`)