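; Passive startup Gameplay Ability that listens for gameplay events under the Attributes tag and turns them into attribute-changing effects on its owner.
; On activation it waits for non-exact tag matches and builds a spec from an event-based Gameplay Effect class.
; It sets the SetByCaller magnitude for the received tag and zeroes every other listed tag to avoid unset-magnitude errors, then applies the spec to itself.
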(event `self.K2_ActivateAbility`
  (bind _returnvalue (`self.GetAbilitySystemComponentFromActorInfo`))
  (`KismetSystemLibrary.PrintString` "监听事件已启动")
  (bind (_asynctaskproxy _payload) (`AbilityTask_WaitGameplayEvent.WaitGameplayEvent` (struct :`TagName` "Attributes") null false false)
    (:`EventReceived`
      (bind (_eventtag _instigator _target _optionalobject _optionalobject2 _contexthandle _instigatortags _targettags _eventmagnitude) (break `GameplayEventData` _payload))
      (set `self.Event Tag` _eventtag)
      (set `self.Event Magnitude` _eventmagnitude)
      (set `self.Spec Handle` (`AbilitySystemComponent.MakeOutgoingSpec` _returnvalue (`self.EnventBasedEffectClass`) 1.0 (`AbilitySystemComponent.MakeEffectContext` _returnvalue)))
      ;[1 1 1] 解决当未设置Tag的振幅值时，报错的问题，设置振幅值（Magnitude)为0
      (for _array_element (`self.Event Tags`)
        (if (`BlueprintGameplayTagLibrary.MatchesTag` _array_element (`self.Event Tag`) true)
          (`AbilitySystemBlueprintLibrary.AssignTagSetByCallerMagnitude` (`self.Spec Handle`) (`self.Event Tag`) (`self.Event Magnitude`))
          (else
            (`AbilitySystemBlueprintLibrary.AssignTagSetByCallerMagnitude` (`self.Spec Handle`) _array_element))))
      (`AbilitySystemComponent.BP_ApplyGameplayEffectSpecToSelf` (`self.GetAbilitySystemComponentFromActorInfo`) (`self.Spec Handle`)))))