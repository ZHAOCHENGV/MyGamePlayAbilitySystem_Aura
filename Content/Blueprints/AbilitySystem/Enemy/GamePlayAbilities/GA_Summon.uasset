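; Enemy Gameplay Ability that has a shaman summon random minions at computed spawn locations.
; On activation it shuffles the locations, plays a ground effect at each and runs the summon montage, ending when the montage completes.
; The montage's gameplay event starts a delayed loop that spawns minions one by one with default controllers.
; Each spawn increments the summoner's minion count, and an OnDestroyed binding decrements it.
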(event `self.K2_ActivateAbility`
  (bind (_output_x _output_y _output_z) (`KismetMathLibrary.BreakVector` (`|GetArrayItem` (`self.SpawnLocation`) (`self.SpawnLocationIndex`))))
  (bind _returnvalue (`self.GetSpawnLocations`))
  (bind _output_get (set `self.SpawnLocation` _returnvalue))
  (`KismetArrayLibrary.Array_Shuffle` _output_get)
  (for _array_element _output_get
    (`NiagaraFunctionLibrary.SpawnSystemAtLocation` "/Game/Assets/Effects/Combat/NS_GroundSummon.NS_GroundSummon" _array_element))
  (`AbilityTask_PlayMontageAndWait.CreatePlayMontageAndWaitProxy` "None" "/Game/Assets/Enemies/Shaman/Animations/Shaman_Summon_Montage.Shaman_Summon_Montage"
    (:`then`
      (`AbilityTask_WaitGameplayEvent.WaitGameplayEvent` (struct :`TagName` "Montage.Attack.1") null
        (:`EventReceived`
          (`KismetSystemLibrary.Delay` 0.2)
          (if (< (`self.SpawnLocationIndex`) (`KismetArrayLibrary.Array_Length` (`self.SpawnLocation`))) :!label _label
            (bind _returnvalue_2 (`|SpawnActorFromClass` (`self.GetRandomMinionClass`) (`KismetMathLibrary.MakeTransform` (`KismetMathLibrary.MakeVector` _output_x _output_y (+ _output_z 50.0)) (`Actor.K2_GetActorRotation` (`self.GetAvatarActorFromActorInfo`))) "Undefined" "MultiplyWithRoot" null null))
            (message `CombatInterface.IncrementMinionCount` (`self.GetAvatarActorFromActorInfo`) 1)
            (add `Actor.OnDestroyed` _returnvalue_2 (delegate `OnDestroyed_事件`))
            (`Pawn.SpawnDefaultController` _returnvalue_2)
            (`/Engine/EditorBlueprintResources/StandardMacros.IncrementInt` (`self.SpawnLocationIndex`)
              (:`  `
                (`KismetSystemLibrary.Delay` 0.2)
                (goto _label)))))))
    (:`OnCompleted`
      (`self.K2_EndAbility`))))

(event `OnDestroyed_事件`
  (params (DestroyedActor :type "Actor Object Reference"))
  (message `CombatInterface.IncrementMinionCount` (`self.GetAvatarActorFromActorInfo`) -1))