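; BP_EnemyBase is the enemy character Blueprint base, handling spawn scale-in, motion-warp facing, dissolve effects and loot drops.
; Timelines drive mesh scale on BeginPlay and the Dissolve parameter on mesh and weapon dynamic materials.
; SpawnLoot rolls items from loot tiers, then a looping timer spawns them one by one at evenly spaced angles and random distances, setting AuraEffectActor level where flagged.
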(event `CombatInterface.UpdateFacingTarget`
  (params (Target :type "Vector Structure (by ref)"))
  (`MotionWarpingComponent.AddOrUpdateWarpTargetFromLocation` (`self.MotionWarping`) "FacingTarget" Target))

(event `self.ReceiveBeginPlay`
  (bind (_direction `_新建轨道_0`) (`Timeline|时间轴`)
    (:`Update`
      (`SceneComponent.SetRelativeScale3D` (`self.Mesh`) (`KismetMathLibrary.Conv_DoubleToVector` `_新建轨道_0`)))))

(event `self.StartDissolveTimeLine`
  (params (DynamicMaterialInstance :type "MaterialInstanceDynamic Object Reference"))
  (bind (_direction `_新建轨道_0`) (`Timeline|溶解网格体时间轴`)
    (:`Update`
      (`MaterialInstanceDynamic.SetScalarParameterValue` DynamicMaterialInstance "Dissolve" `_新建轨道_0`))))

(event `self.StartWeaponDissolveTimeLine`
  (params (DynamicMaterialInstance :type "MaterialInstanceDynamic Object Reference"))
  (bind (_direction `_新建轨道_0`) (`Timeline|溶解武器时间轴`)
    (:`Update`
      (`MaterialInstanceDynamic.SetScalarParameterValue` DynamicMaterialInstance "Dissolve" `_新建轨道_0`))))

(event `self.SpawnLoot`
  (bind _returnvalue (`AuraAbilitySystemLibrary.GetLootTiers` null))
  (`/Engine/EditorBlueprintResources/StandardMacros.IsValid` _returnvalue
    (:`Is Valid`
      (bind _returnvalue_2 (`LootTiers.GetLootItems` _returnvalue))
      (bind _output_get (set `self.LootItems` _returnvalue_2))
      (set `self.LootRotations` (`self.Get Loot Rotations` _output_get))
      (bind _returnvalue_3 (`KismetSystemLibrary.K2_SetTimerDelegate` (delegate `生成战利品`) 0.1 true))
      (set `self.LootTimer` _returnvalue_3)
      (`self.生成战利品`))))

(event `生成战利品`
  (bind (_lootclass _blootleveloverride) (break `LootItem` (`|GetArrayItem` (`self.LootItems`) (`self.SpawnLoopCount`))))
  (if (< (`self.SpawnLoopCount`) (`KismetArrayLibrary.Array_Length` (`self.LootItems`)))
    (bind _returnvalue (`|SpawnActorFromClass` _lootclass (`self.NewFunction` (`self.SpawnLoopCount`)) "AdjustIfPossibleButAlwaysSpawn" "MultiplyWithRoot" null null))
    (`/Engine/EditorBlueprintResources/StandardMacros.IsValid` _returnvalue
      (:`Is Valid`
        (bind _asaura_effect_actor (cast `AuraEffectActor` _returnvalue)
          (:`then`
            (if _blootleveloverride
              (set `AuraEffectActor.ActorLevel` (`KismetMathLibrary.Conv_IntToDouble` (`self.Level`)) _asaura_effect_actor)))
          (:`CastFailed`
            _))
        (`/Engine/EditorBlueprintResources/StandardMacros.IncrementInt` (`self.SpawnLoopCount`))))
    (else
      (`KismetSystemLibrary.K2_ClearAndInvalidateTimerHandle` (`self.LootTimer`)))))

(fn `Get Loot Rotations`
  (params (TargetArray :type "Array of LootItem Structure (by ref)"))
  (returns (ReturnValue :type "Array of Rotator Structure"))
  (return (`AuraAbilitySystemLibrary.EvenlySpacedRotators` (`self.GetActorForwardVector`) (`KismetMathLibrary.Vector_Up`) 360.0 (`KismetArrayLibrary.Array_Length` TargetArray))))

(fn `NewFunction`
  (params (LoopCount :type Integer))
  (returns (SpawnTransform :type "Transform Structure"))
  (bind _output (`|GetArrayItem` (`self.LootRotations`) LoopCount))
  (return (`KismetMathLibrary.MakeTransform` (+ (* (`KismetMathLibrary.GetForwardVector` _output) (`KismetMathLibrary.RandomFloatInRange` (`self.MinSpawnDistance`) (`self.MaxSpawnDistance`))) (`self.K2_GetActorLocation`)) _output)))

(fn `UserConstructionScript`)